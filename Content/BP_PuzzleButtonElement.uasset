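; BP_PuzzleButtonElement is a clickable colored button that submits guesses to a puzzle.
; On BeginPlay it creates a dynamic instance of M_Colorable, applies it to its Plane and sets its color.
; Clicking turns on the material's Highlight parameter; releasing turns it off and passes the button's Index to the referenced Puzzle's Guess.
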(event `self.ReceiveBeginPlay`
  (bind _returnvalue (`KismetMaterialLibrary.CreateDynamicMaterialInstance` "/Game/M_Colorable.M_Colorable"))
  (`PrimitiveComponent.SetMaterial` (`self.Plane`) 0 _returnvalue)
  (`MaterialInstanceDynamic.SetVectorParameterValue` _returnvalue "Color" (`self.Color`))
  (set `self.Material` _returnvalue))

(event `self.ReceiveActorOnClicked`
  (params (ButtonPressed :type "Key Structure"))
  (`self.Highlight` true))

(event `self.ReceiveActorOnReleased`
  (params (ButtonReleased :type "Key Structure"))
  (`self.Highlight` false)
  (`Puzzle.Guess` (`self.Puzzle`) (`self.Index`)))

(event `self.Highlight`
  (params (bIsHighlight :type Boolean))
  (bind _material (`self.Material`))
  (if bIsHighlight
    (`MaterialInstanceDynamic.SetScalarParameterValue` _material "Highlight" 1.0)
    (else
      (`MaterialInstanceDynamic.SetScalarParameterValue` _material "Highlight" 0.0))))

(fn `UserConstructionScript`)